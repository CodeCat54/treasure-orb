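; BP_PhysicsTrophy is a gold statue trophy actor that fades out and destroys itself when it falls off the map.
; BeginPlay creates and stores dynamic material instances for the statue mesh's platform base and gold metal slots.
; The DeathPlane event plays a timeline that drives the Opacity parameter on both instances, then destroys the actor when finished.
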(event `self.ReceiveBeginPlay`
  ;[1 1 1] Initalise dynamic materials
  (bind _returnvalue (`PrimitiveComponent.CreateDynamicMaterialInstance` (`self.StatueMesh`) 0 "/Game/Materials/M_AssetPlatform.M_AssetPlatform" "None"))
  (set `self.DynamicMaterialBase` _returnvalue)
  (bind _returnvalue_2 (`PrimitiveComponent.CreateDynamicMaterialInstance` (`self.StatueMesh`) 1 "/Game/Materials/M_Metal_Gold.M_Metal_Gold" "None"))
  (set `self.DynamicMaterialStatue` _returnvalue_2))

(event `/Game/Interfaces/I_Interaction.DeathPlane`
  ;[1 1 1] Fade out when falling off map
  (bind (_direction _opacity) (`Timeline|OpacityTimeline`)
    (:`Update`
      (`MaterialInstanceDynamic.SetScalarParameterValue` (`self.DynamicMaterialBase`) "Opacity" _opacity)
      (`MaterialInstanceDynamic.SetScalarParameterValue` (`self.DynamicMaterialStatue`) "Opacity" _opacity))
    (:`Finished`
      (`self.K2_DestroyActor`))))

(fn `UserConstructionScript`)