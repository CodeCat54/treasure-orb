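; BP_Trophy is a spinning pickup that awards a level trophy and flags the final one.
; A self-restarting timeline drives its yaw through full turns.
; On first overlap with an actor implementing I_Interaction, it sends TrophyPickupMessage with audio selected by TrophyNum and a final-trophy flag, then destroys itself.
; The receiving actor is left to handle the audio and any end-of-game response.
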(event `ResetRotation`
  (bind (_returnvalue_roll _returnvalue_pitch) (`KismetMathLibrary.BreakRotator` (`self.K2_GetActorRotation`)))
  ;[1 1 1] Spin in circles
  (bind (_direction _rotation) (`Timeline|RotationTimeline` :!via `PlayFromStart` :!label _label)
    (:`Update`
      (`self.K2_SetActorRotation` (`KismetMathLibrary.MakeRotator` _returnvalue_roll _returnvalue_pitch (* _rotation 360.0))))
    (:`Finished`
      (`self.ResetRotation`))))

(event `self.ReceiveBeginPlay`
  ;[1 1 1] Spin in circles
  (goto _label :!via `PlayFromStart`))

(event `self.ReceiveActorBeginOverlap`
  (params (OtherActor :type "Actor Object Reference"))
  (bind _trophynum (`self.TrophyNum`))
  ;[1 1 1] Give player correct audio on interaction, end game if final trophy
  (if (`KismetSystemLibrary.DoesImplementInterface` OtherActor "/Game/Interfaces/I_Interaction.I_Interaction_C")
    (`/Engine/EditorBlueprintResources/StandardMacros.DoOnce` false
      (:`Completed`
        (message `/Game/Interfaces/I_Interaction.TrophyPickup` OtherActor (select `int` _trophynum :`0` "/Game/Sounds/MSC_Level1.MSC_Level1" :`1` "/Game/Sounds/MSC_Level2.MSC_Level2" :`2` "/Game/Sounds/MSC_Level3.MSC_Level3" :`3` "/Game/Sounds/MSC_Level4.MSC_Level4" :`4` "/Game/Sounds/MSC_Win.MSC_Win" :!type "SoundBase Object Reference") (== _trophynum 4))
        (`self.K2_DestroyActor`)))))

(fn `UserConstructionScript`)